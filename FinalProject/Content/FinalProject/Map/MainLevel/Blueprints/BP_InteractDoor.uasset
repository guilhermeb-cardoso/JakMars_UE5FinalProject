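; BP_InteractDoor is an interactable door that swings open and closed when FnInteract fires while the player is in range.
; Box overlaps with BPI_Player actors toggle input and CanOpen.
; The DoorRot timeline drives mesh yaw forward or in reverse, playing a sound once per swing and flipping IsDoorClosed when finished.
; A prompt text yaws toward the player, shows only within a set distance, and stays hidden after first use.
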(event `self.ReceiveTick`
  (params (DeltaSeconds :type "Float (single-precision)"))
  (bind _textrender (`self.TextRender`))
  (bind _textrender_2 (`self.TextRender`))
  (bind (_returnvalue_roll _returnvalue_pitch _returnvalue_yaw) (`KismetMathLibrary.BreakRotator` (`KismetMathLibrary.FindLookAtRotation` (`SceneComponent.K2_GetComponentLocation` _textrender) (`self.K2_GetActorLocation` (`GameplayStatics.GetPlayerPawn` 0)))))
  (`SceneComponent.K2_SetWorldRotation` _textrender (`KismetMathLibrary.MakeRotator` 0.0 0.0 _returnvalue_yaw) false false) ; Makes so the Text is Always \nturned Towards the player
  (if (`self.EPressed`)
    _
    (elif (> (`self.GetDistanceTo` (`GameplayStatics.GetPlayerPawn` 0)) 1000.0)
      (`SceneComponent.SetVisibility` _textrender_2 false false) ; Invisible
      (else
        (`SceneComponent.SetVisibility` _textrender_2 true false) ; Visible
      ))))

(event `self.Box.OnComponentBeginOverlap`
  (params (OverlappedComponent :type "PrimitiveComponent Object Reference") (OtherActor :type "Actor Object Reference") (OtherComp :type "PrimitiveComponent Object Reference") (OtherBodyIndex :type Integer) (bFromSweep :type Boolean) (SweepResult :type "HitResult Structure (by ref)"))
  (if (`KismetSystemLibrary.DoesImplementInterface` OtherActor "/Game/FinalProject/BlueprintInterfaces/Player/BPI_Player.BPI_Player_C")
    (`self.EnableInput` (`GameplayStatics.GetPlayerController` 0))
    (set `self.CanOpen` true)))

(event `self.Box.OnComponentEndOverlap`
  (params (OverlappedComponent :type "PrimitiveComponent Object Reference") (OtherActor :type "Actor Object Reference") (OtherComp :type "PrimitiveComponent Object Reference") (OtherBodyIndex :type Integer))
  (if (`KismetSystemLibrary.DoesImplementInterface` OtherActor "/Game/FinalProject/BlueprintInterfaces/Player/BPI_Player.BPI_Player_C")
    (`self.DisableInput` (`GameplayStatics.GetPlayerController` 0))
    (set `self.CanOpen` false)))

(event `/Game/FinalProject/BlueprintInterfaces/Interactables/BPI_Interact.Fn_Interact`
  (if (`self.CanOpen`)
    (if (`self.IsDoorClosed`)
      (bind (_direction _dooropen) (`Timeline|DoorRot` :!label _label)
        (:`Update`
          (`SceneComponent.K2_SetRelativeRotation` (`self.StaticMesh`) (`KismetMathLibrary.MakeRotator` 0.0 0.0 _dooropen) false false)
          (`SceneComponent.SetVisibility` (`self.TextRender`) false false) ; Invisible
          (set `self.EPressed` true)
          (`/Engine/EditorBlueprintResources/StandardMacros.DoOnce` false :!label _label_2
            (:`Completed`
              (`GameplayStatics.PlaySound2D` "/Game/FinalProject/Sounds/Level/DoorOpening_Cue.DoorOpening_Cue" 1.0 1.0 0.0 null null))))
        (:`Finished`
          (if (`self.IsDoorClosed`)
            (set `self.IsDoorClosed` false)
            (goto _label_2 :!via `Reset`)
            (else
              (set `self.IsDoorClosed` true)
              (goto _label_2 :!via `Reset`)))))
      (else
        (goto _label :!via `ReverseFromEnd`)))))

(fn `UserConstructionScript`)