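; Rifle-armed enemy AI character that patrols, shoots the player, reacts to hits and ragdolls on death.
; Sighting the player or getting hit alerts all BPI_Enemy actors at once.
; Tick checks player life and sphere-traced sight within a randomized range, feeding Blackboard keys, and updates a player-facing HP bar.
; Shots apply damage through a line trace to a random point around the player, with CompShoot spawning a short-lived bullet.
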(event `self.ReceiveBeginPlay`
  (`self.EV_AiMovSpeed`))

(event `self.ReceiveTick`
  (params (DeltaSeconds :type "Float (single-precision)"))
  (`self.EV_AiMovSpeed`)
  (`self.FN_IsPlayeAlive`)
  (`self.FN_SetWidgetRotation`)
  (`self.FN_UpdateHPBar`)
  (`self.Can Shoot`))

(event `self.PawnSensing.OnSeePawn`
  (params (Pawn :type "Pawn Object Reference"))
  ;[0 0 0] Enemy sees Player
  (message `/Game/FinalProject/BlueprintInterfaces/Player/BPI_Player.GetPlayerRef` Pawn) ; BPI to get Player Ref
  (bind _outactors (`GameplayStatics.GetAllActorsWithInterface` "/Game/FinalProject/BlueprintInterfaces/Enemy/BPI_Enemy.BPI_Enemy_C"))
  (message `/Game/FinalProject/BlueprintInterfaces/Enemy/BPI_Enemy.FN_EnKnowPlayerPos` _outactors))

(event `EV_AiMovSpeed`
  (bind _charactermovement (`self.CharacterMovement`))
  ;[0 0 0] Movement Speed
  (if (`self.hasSeenPlayer`)
    (set `CharacterMovementComponent.MaxWalkSpeed` 300.0 _charactermovement)
    (else
      (set `CharacterMovementComponent.MaxWalkSpeed` 200.0 _charactermovement))))

(event `/Game/FinalProject/BlueprintInterfaces/Enemy/BPI_Enemy.FN_EnShootAnim`
  ;[0 0 0] Plays Shooting animation
  (message `/Game/FinalProject/BlueprintInterfaces/Enemy/BPI_EnAnim.FN_PlayEnShoot` (`SkeletalMeshComponent.GetAnimInstance` (`self.Mesh`)) 5.0 true))

(event `/Game/FinalProject/BlueprintInterfaces/Enemy/BPI_Enemy.FN_EnemyShoot`
  (bind _gunarrow (`self.GunArrow`))
  (bind _returnvalue (`SceneComponent.K2_GetComponentLocation` _gunarrow))
  ;[0 0 0] Shooting
  (bind _outhit (`KismetSystemLibrary.LineTraceSingle` :`Start` (`SceneComponent.K2_GetComponentLocation` (`self.GunArrow`)) :`End` (`KismetMathLibrary.RandomPointInBoundingBox` (`self.K2_GetActorLocation` (`GameplayStatics.GetPlayerCharacter` 0)) (100.0 100.0 100.0)) :`TraceChannel` "TraceTypeQuery2" :`TraceColor` (struct :`G` 0.675999 :`B` 1.0 :`A` 1.0) :`TraceHitColor` (struct :`R` 1.0 :`G` 0.851476 :`A` 1.0) :`DrawTime` 0.3))
  (`|ExecutionSequence`
    (:`then_0`
      (bind _bullet (`/Game/FinalProject/Components/Comp_Shoot.FN_Shoot` (`self.Comp_Shoot`) _returnvalue (`.TraceEnd` (`GameplayStatics.BreakHitResult` _outhit)))) ; Shoots Bullet
      (bind _output_get (set `self.Bullet` _bullet))
      (`/Engine/EditorBlueprintResources/StandardMacros.IsValid` _output_get
        (:`Is Valid`
          (`GameplayStatics.SpawnEmitterAtLocation` "/Game/FinalProject/Player/Weapon/Ak47/Vfx/P_Explosion_Big_C.P_Explosion_Big_C" _returnvalue (`SceneComponent.K2_GetComponentRotation` _gunarrow) (0.3 0.3 0.3)) ; Shooting VFX
          (`GameplayStatics.SpawnEmitterAtLocation` "/Game/Realistic_Starter_VFX_Pack_Vol2/Particles/Blood/P_Blood_Splat_Cone.P_Blood_Splat_Cone" (`.ImpactPoint` (`GameplayStatics.BreakHitResult` _outhit)) (`KismetMathLibrary.Conv_VectorToRotator` (`SceneComponent.GetUpVector` (`Actor.RootComponent` (`self.Bullet`)))) (0.5 0.5 0.5)) ; Blood VFX if Hits Player
          (`self.SetLifeSpan` (`self.Bullet`) 0.2))))
    (:`then_1`
      (if (`KismetSystemLibrary.DoesImplementInterface` (`.HitActor` (`GameplayStatics.BreakHitResult` _outhit)) "/Game/FinalProject/BlueprintInterfaces/Player/BPI_Player.BPI_Player_C")
        (`GameplayStatics.ApplyDamage` (`.HitActor` (`GameplayStatics.BreakHitResult` _outhit)) 5.0)))))

(event `/Game/FinalProject/BlueprintInterfaces/Death/BPI_Death.Death`
  ;[0 0 0] Death
  (message `/Game/FinalProject/BlueprintInterfaces/Enemy/BPI_EnAnim.FN_PlayEnDeath` (`SkeletalMeshComponent.GetAnimInstance` (`self.Mesh`)))
  (set `self.EnIsDead` true)
  (set `CharacterMovementComponent.MaxWalkSpeed` 0.0 (`self.CharacterMovement`))
  (`BlackboardComponent.SetValueAsBool` (`AIBlueprintHelperLibrary.GetBlackboard` (`AIBlueprintHelperLibrary.GetAIController` self)) "EnIsDead" true) ; Set Bool as true
  (`PrimitiveComponent.SetCollisionEnabled` (`self.CapsuleComponent`) "NoCollision")
  (`PrimitiveComponent.SetSimulatePhysics` (`self.Rifle`) true)
  (`PrimitiveComponent.SetSimulatePhysics` (`self.Mesh`) true)
  (`self.SetLifeSpan` 15.0))

(event `/Game/FinalProject/BlueprintInterfaces/Death/BPI_Death.FN_GotHit`
  (bind _returnvalue (`AIBlueprintHelperLibrary.GetBlackboard` (`AIBlueprintHelperLibrary.GetAIController` self)))
  ;[0 0 0] Hit
  (message `/Game/FinalProject/BlueprintInterfaces/Enemy/BPI_EnAnim.FN_PlayEnHit` (`SkeletalMeshComponent.GetAnimInstance` (`self.Mesh`))) ; Hit Animation
  (`BlackboardComponent.SetValueAsBool` _returnvalue "EnGotHit" true) ; Set Bool as true
  (set `CharacterMovementComponent.MaxWalkSpeed` 0.0 (`self.CharacterMovement`))
  (`KismetSystemLibrary.Delay` 0.97)
  (`BlackboardComponent.SetValueAsBool` _returnvalue "EnGotHit" false) ; Set Bool as false
  (`self.EV_AiMovSpeed`)
  (`BlackboardComponent.SetValueAsBool` _returnvalue "HasSeenPlayer" true) ; Set Bool as true
  (bind _outactors (`GameplayStatics.GetAllActorsWithInterface` "/Game/FinalProject/BlueprintInterfaces/Enemy/BPI_Enemy.BPI_Enemy_C"))
  (message `/Game/FinalProject/BlueprintInterfaces/Enemy/BPI_Enemy.FN_EnKnowPlayerPos` _outactors))

(event `Can Shoot`
  (bind _returnvalue (`AIBlueprintHelperLibrary.GetBlackboard` (`AIBlueprintHelperLibrary.GetAIController` self)))
  ;[0 0 0] Is Player in Sight
  (if (`self.EnIsDead`)
    _
    (elif (`self.hasSeenPlayer`)
      (bind _outhit (`KismetSystemLibrary.SphereTraceSingle` :`Start` (`self.K2_GetActorLocation`) :`End` (`self.K2_GetActorLocation` (`GameplayStatics.GetPlayerCharacter` 0)) :`Radius` 25.0 :`TraceChannel` "TraceTypeQuery1" :`DrawDebugType` "ForOneFrame"))
      (if (< (`self.GetDistanceTo` (`GameplayStatics.GetPlayerCharacter` 0)) (`KismetMathLibrary.RandomFloatInRange` 500.0 1000.0))
        (if (`KismetSystemLibrary.DoesImplementInterface` (`.HitActor` (`GameplayStatics.BreakHitResult` _outhit)) "/Game/FinalProject/BlueprintInterfaces/Player/BPI_Player.BPI_Player_C")
          (`BlackboardComponent.SetValueAsBool` _returnvalue "CanShoot" true) ; Set Bool as true
          (set `CharacterMovementComponent.MaxWalkSpeed` 0.0 (`self.CharacterMovement`))
          (else
            (`BlackboardComponent.SetValueAsBool` _returnvalue "CanShoot" false) ; Set Bool as false
            (`self.EV_AiMovSpeed`)))))))

(fn `FN_EnGetEnemyRef`
  (returns (EnemyRef :type "/Game/FinalProject/Enemy/Character/BP_Enemy1 Object Reference"))
  (return self))

(fn `FN_EnHasSeenPlayer`
  (returns (`EnHasSeenPlayer?` :type Boolean))
  (return (`self.hasSeenPlayer`)))

(fn `FN_EnKnowPlayerPos`
  (returns (SawPlayer :type Boolean))
  (bind _output_get (set `self.hasSeenPlayer` true))
  (`BlackboardComponent.SetValueAsBool` (`AIBlueprintHelperLibrary.GetBlackboard` (`AIBlueprintHelperLibrary.GetAIController` self)) "HasSeenPlayer" _output_get) ; Set Bool as true
  (return _output_get))

(fn `FN_GetPatrolPoints`
  (returns (PatrolPointsOut :type "Array of Vector Structure"))
  (return (`self.PatrolPoints`)))

(fn `FN_IsPlayeAlive`
  (bind _returnvalue (`AIBlueprintHelperLibrary.GetBlackboard` (`AIBlueprintHelperLibrary.GetAIController` self)))
  (bind _isplayeralive (message `/Game/FinalProject/BlueprintInterfaces/Player/BPI_Player.IsPlayerAlive` (`GameplayStatics.GetPlayerCharacter` 0)))
  (if _isplayeralive
    (`BlackboardComponent.SetValueAsBool` _returnvalue "PlayerIsAlive" true) ; Set Bool as true
    (else
      (`BlackboardComponent.SetValueAsBool` _returnvalue "PlayerIsAlive" false) ; Set Bool as true
      (bind _asabp_enemy (cast `/Game/FinalProject/Enemy/Animation/ABP_Enemy` (`SkeletalMeshComponent.GetAnimInstance` (`self.Mesh`))))
      (`/Engine/EditorBlueprintResources/StandardMacros.IsValid` _asabp_enemy
        (:`Is Valid`
          (set `/Game/FinalProject/Enemy/Animation/ABP_Enemy.Shoot` false _asabp_enemy))))))

(fn `FN_SetPatrolPoints`
  (params (PatrolPointsIn :type "Array of Vector Structure (by ref)"))
  (set `self.PatrolPoints` PatrolPointsIn)
  (return))

(fn `FN_SetWidgetRotation`
  (`SceneComponent.K2_SetWorldRotation` (`self.HpBar`) (`KismetMathLibrary.FindLookAtRotation` (`self.K2_GetActorLocation`) (`self.K2_GetActorLocation` (`GameplayStatics.GetPlayerCharacter` 0))) false false) ; Rotates Towards Player
)

(fn `FN_UpdateHPBar`
  (bind _comp_life (`self.Comp_Life`))
  (bind _aswbp_enemy_ui (cast `/Game/FinalProject/Enemy/UI/WBP_EnemyUI` (`WidgetComponent.GetWidget` (`self.HpBar`))))
  (`/Engine/EditorBlueprintResources/StandardMacros.IsValid` _aswbp_enemy_ui
    (:`Is Valid`
      (bind _enemyhpbar (`/Game/FinalProject/Enemy/UI/WBP_EnemyUI.EnemyHpBar` _aswbp_enemy_ui))
      (`ProgressBar.SetPercent` _enemyhpbar (`KismetMathLibrary.SafeDivide` (`/Game/FinalProject/Components/Comp_Life.HP` _comp_life) (`/Game/FinalProject/Components/Comp_Life.MaxHP` _comp_life)))
      (if (`BlackboardComponent.GetValueAsBool` (`AIBlueprintHelperLibrary.GetBlackboard` (`AIBlueprintHelperLibrary.GetAIController` self)) "EnIsDead")
        (`Widget.SetVisibility` _enemyhpbar "Collapsed")))))

(fn `UserConstructionScript`
  (`SkinnedMeshComponent.SetLeaderPoseComponent` (`self.Feet`) (`self.Mesh`) true false)
  (`SkinnedMeshComponent.SetLeaderPoseComponent` (`self.Legs`) (`self.Mesh`) true false)
  (`SkinnedMeshComponent.SetLeaderPoseComponent` (`self.Torso`) (`self.Mesh`) true false)
  (`SkinnedMeshComponent.SetLeaderPoseComponent` (`self.Body`) (`self.Mesh`) true false)
  (`SkinnedMeshComponent.SetLeaderPoseComponent` (`self.Face`) (`self.Mesh`) true false))