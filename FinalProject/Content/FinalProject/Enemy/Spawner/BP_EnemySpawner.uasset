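; BP_EnemySpawner is a one-shot trigger that spawns patrolling enemies when an actor implementing BPI_Player enters its box.
; A DoN gate starts a loop that spawns a BP_Enemy1 at each SpawnTransform and sends it the shared PatrolPoints by message.
; The spawner destroys itself after a short delay.
; SpawnTransforms are used directly as world transforms, so the spawner must sit at the origin while they are chosen.
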(event `self.ReceiveBeginPlay`)

(event `self.Box.OnComponentBeginOverlap`
  (params (OverlappedComponent :type "PrimitiveComponent Object Reference") (OtherActor :type "Actor Object Reference") (OtherComp :type "PrimitiveComponent Object Reference") (OtherBodyIndex :type Integer) (bFromSweep :type Boolean) (SweepResult :type "HitResult Structure (by ref)"))
  (bind _spawn_transform (`self.Spawn Transform`))
  (if (`KismetSystemLibrary.DoesImplementInterface` OtherActor "/Game/FinalProject/BlueprintInterfaces/Player/BPI_Player.BPI_Player_C")
    (`/Engine/EditorBlueprintResources/StandardMacros.Do N` 1
      (:`Exit`
        (for _index (range (+ (`KismetArrayLibrary.Array_LastIndex` _spawn_transform) 1))
          (bind _returnvalue (`|SpawnActorFromClass` "/Game/FinalProject/Enemy/Character/BP_Enemy1.BP_Enemy1_C" (`|GetArrayItem` _spawn_transform _index) "AlwaysSpawn" "MultiplyWithRoot" null null)) ; Spawner Must be at 0 x 0 x 0 when choosing the the SpawnTransforms
          (bind _output_get (set `self.EnemyRef` _returnvalue))
          (`/Engine/EditorBlueprintResources/StandardMacros.IsValid` _output_get
            (:`Is Valid`
              (message `/Game/FinalProject/BlueprintInterfaces/Enemy/BPI_Enemy.FN_SetPatrolPoints` _output_get (`self.PatrolPoints`))
              (`KismetSystemLibrary.Delay` 0.2)
              (`self.K2_DestroyActor`))))))))

(fn `UserConstructionScript`)