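; Player controller for the main game mode that registers the main character's Enhanced Input mapping context and handles pausing.
; On BeginPlay it adds the mapping context, and the pause input action calls a toggle function.
; That function finds the HUD actor by class to reach its pause menu widget, then flips game pause, menu visibility, mouse cursor and input mode together.
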(event `self.ReceiveBeginPlay`
  (bind _returnvalue (subsystem `EnhancedInputLocalPlayerSubsystem`))
  (`/Engine/EditorBlueprintResources/StandardMacros.IsValid` _returnvalue
    (:`Is Valid`
      (`EnhancedInputSubsystemInterface.AddMappingContext` _returnvalue "/Game/FinalProject/Player/Input/IMC_MainCharacter.IMC_MainCharacter" 0 (struct)))))

(event `self.ReceiveTick`
  (params (DeltaSeconds :type "Float (single-precision)")))

(event `EnhancedInput|/Game/FinalProject/Player/Input/InputAction/IA_MCPauseGame`
  (params (ActionValue :type Boolean) (ElapsedSeconds :type "Float (double-precision)") (TriggeredSeconds :type "Float (double-precision)") (InputAction :type "InputAction Object Reference" :default "/Game/FinalProject/Player/Input/InputAction/IA_MCPauseGame.IA_MCPauseGame"))
  (:`Started`
    (`self.Fn_HandlePause`) ; Pause/Unpause Game
  ))

(fn `Fn_HandlePause`
  (bind _returnvalue (`GameplayStatics.GetPlayerController` 0))
  (bind _pause_menu_widget (`self.Pause Menu Widget`))
  (bind _returnvalue_2 (`GameplayStatics.GetActorOfClass` "/Game/FinalProject/UI/Player/BP_PlayerHUD.BP_PlayerHUD_C"))
  (set `self.Pause Menu Widget` (`/Game/FinalProject/UI/Player/BP_PlayerHUD.PauseMenuWidget` _returnvalue_2))
  (if (`GameplayStatics.IsGamePaused`)
    (`GameplayStatics.SetGamePaused` false)
    (`Widget.SetVisibility` _pause_menu_widget "Collapsed")
    (set `PlayerController.bShowMouseCursor` false _returnvalue)
    (`WidgetBlueprintLibrary.SetInputMode_GameOnly` _returnvalue)
    (else
      (`GameplayStatics.SetGamePaused` true)
      (`Widget.SetVisibility` _pause_menu_widget "Visible")
      (set `PlayerController.bShowMouseCursor` true _returnvalue)
      (`WidgetBlueprintLibrary.SetInputMode_GameAndUIEx` _returnvalue (`self.Pause Menu Widget`) "LockInFullscreen"))))

(fn `UserConstructionScript`)